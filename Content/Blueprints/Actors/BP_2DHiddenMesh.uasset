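; BP_2DHiddenMesh is an actor whose static mesh exists only in the 3D view and disappears when the game switches to 2D.
; On BeginPlay it binds to the BP_Gamemode ChangeViewTo2D and ChangeViewTo3D dispatchers.
; The 2D event hides the mesh and disables its collision, while the 3D event shows it and restores query and physics collision.
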(event Custom|ChangeViewTo2D
  (params (ViewPlane :type Vector%204%20Structure) (Distanse :type Float%20%28single-precision%29))
  (bind _staticmesh (Variables|Default|GetStaticMesh))
  (Development|SetHiddeninGame _staticmesh true false)
  (Collision|SetCollisionEnabled _staticmesh "NoCollision"))

(event Custom|ChangeViewTo3D
  (params (Character :type BP%203D%20Character%20Object%20Reference))
  (bind _staticmesh (Variables|Default|GetStaticMesh))
  (Development|SetHiddeninGame _staticmesh false false)
  (Collision|SetCollisionEnabled _staticmesh "QueryAndPhysics"))

(event EventBeginPlay
  (bind _asbp_gamemode (Utilities|Casting|CastToBP_Gamemode (Game|GetGameMode)))
  (EventDispatchers|AssignChangeViewto2D _asbp_gamemode (delegate Custom|ChangeViewTo2D))
  (EventDispatchers|AssignChangeViewto3D _asbp_gamemode (delegate Custom|ChangeViewTo3D)))

(event Collision|EventActorBeginOverlap
  (params (OtherActor :type Actor%20Object%20Reference)))

(event EventTick
  (params (DeltaSeconds :type Float%20%28single-precision%29)))

(fn ConstructionScript)