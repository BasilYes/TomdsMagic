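; BP_2DButtonLVL1 is an interactable button that a 2D character uses to switch the game to 3D.
; On BeginPlay it caches the first actor tagged "Out" as its ActionActor.
; Interact casts the owner to BP_2DCharacter and the game mode to BP_Gamemode, calls ChangeTo3D, sends ActionMessage to that actor and turns the button green.
; It returns true on success and false if either cast fails.
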(event EventBeginPlay
  (|CallParentFunction)
  (bind _outactors (Actor|GetAllActorswithTag "Out"))
  (Variables|Default|SetActionActor (Utilities|Array|Get(acopy) _outactors)))

(event Collision|EventActorBeginOverlap
  (params (OtherActor :type Actor%20Object%20Reference))
  (|CallParentFunction OtherActor) ; This node is disabled and will not be called.\nDrag off pins to build functionality.
)

(event EventTick
  (params (DeltaSeconds :type Float%20%28single-precision%29))
  (|CallParentFunction DeltaSeconds) ; This node is disabled and will not be called.\nDrag off pins to build functionality.
)

(fn ConstructionScript
  (|CallParentFunction))

(fn Interact
  (params (owner :type Pawn%20Object%20Reference))
  (bind _asbp_2dcharacter (Utilities|Casting|CastToBP_2DCharacter owner)
    (:then
      (bind _asbp_gamemode (Utilities|Casting|CastToBP_Gamemode (Game|GetGameMode))
        (:then
          (Default|Changeto3D _asbp_gamemode _asbp_2dcharacter)
          (Class|INAction|Action(Message) (Variables|Default|GetActionActor))
          (Rendering|Material|SetMaterial (Variables|Default|GetboxModel) 0 "/Game/Materials/M_Green.M_Green")
          (return true))
        (:CastFailed
          (return false))))
    (:CastFailed
      (return false))))