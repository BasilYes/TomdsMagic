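; Interactable wall eye that switches the game between 3D and 2D views through BP_Gamemode.
; Interact sends a 3D character to 2D only if its LegsButton is valid, and returns a 2D character to 3D.
; Gamemode view-change callbacks swap the sprite between open in 3D and not open in 2D.
; Prompt text follows the current view, with a temporary failure message driven by FailInteraction's retriggerable delay.
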(event Custom|ChangeViewTo2D_Event_0
  (params (ViewPlane :type Vector%204%20Structure) (Distanse :type Float%20%28single-precision%29))
  (Rendering|Components|Sprite|SetSprite (Variables|Default|GetPaperSprite) "/Game/Brush/SP_WallEyeNotOpen.SP_WallEyeNotOpen"))

(event Custom|ChangeViewTo3D_Event_0
  (params (Character :type BP%203D%20Character%20Object%20Reference))
  (Rendering|Components|Sprite|SetSprite (Variables|Default|GetPaperSprite) "/Game/Brush/SP_WallEyeOpen.SP_WallEyeOpen"))

(event EventBeginPlay
  (bind _asbp_gamemode (Utilities|Casting|CastToBP_Gamemode (Game|GetGameMode)))
  (EventDispatchers|AssignChangeViewto2D _asbp_gamemode (delegate Custom|ChangeViewTo2D_Event_0))
  (EventDispatchers|AssignChangeViewto3D _asbp_gamemode (delegate Custom|ChangeViewTo3D_Event_0)))

(event Collision|EventActorBeginOverlap
  (params (OtherActor :type Actor%20Object%20Reference)))

(event EventTick
  (params (DeltaSeconds :type Float%20%28single-precision%29)))

(event EventFailInteraction
  (Variables|Default|SetIsFail true)
  (Utilities|FlowControl|RetriggerableDelay 2.0)
  (Variables|Default|SetIsFail false))

(fn ConstructionScript)

(fn GetInteractionText
  (bind _asbp_gamemode (Utilities|Casting|CastToBP_Gamemode (Game|GetGameMode)))
  (return (select (Variables|/Game/Blueprints/GameRules/BP_Gamemode.BP_Gamemode_C|GetIs2D _asbp_gamemode) "Вернуться" (select (Variables|Default|GetIsFail) "Ничего не произошло" "Присмотреться")) (Variables|Default|GetIsFail)))

(fn Interact
  (params (owner :type Pawn%20Object%20Reference))
  (bind _asbp_3dcharacter (Utilities|Casting|CastToBP_3DCharacter owner)
    (:then
      (Utilities|IsValid (Variables|/Game/Blueprints/Characters/BP_3DCharacter.BP_3DCharacter_C|GetLegsButton _asbp_3dcharacter)
        (:Is%20Valid
          (bind _asbp_gamemode (Utilities|Casting|CastToBP_Gamemode (Game|GetGameMode))
            (:then
              (Default|Changeto2D _asbp_gamemode self)
              (return true))
            (:CastFailed
              (return false))))
        (:Is%20Not%20Valid
          (return false))))
    (:CastFailed
      (bind _asbp_2dcharacter (Utilities|Casting|CastToBP_2DCharacter owner)
        (:then
          (bind _asbp_gamemode_2 (Utilities|Casting|CastToBP_Gamemode (Game|GetGameMode)))
          (Default|Changeto3D _asbp_gamemode_2 _asbp_2dcharacter)
          (return true))
        (:CastFailed
          (return false))))))