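; BP_2DButton is an interactable button that a BP_2DCharacter presses to send ActionMessage to its linked ActionActor.
; Interact rejects other users and repeat presses, otherwise turns the box green and sets Pressed, which also switches the Russian prompt to a failed "pressed" state.
; A positive UnpressTimer makes it a timed button: blue from BeginPlay and reset after that delay, while otherwise it stays pressed.
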(event Custom|PressEvent
  (if (> (Variables|Default|GetunpressTimer) 0.0)
    (Utilities|FlowControl|Delay (Variables|Default|GetunpressTimer))
    (Rendering|Material|SetMaterial (Variables|Default|GetboxModel) 0 "/Game/Materials/M_Blue.M_Blue")
    (Variables|Default|SetPressed false)))

(event EventBeginPlay
  (if (> (Variables|Default|GetunpressTimer) 0.0)
    (Rendering|Material|SetMaterial (Variables|Default|GetboxModel) 0 "/Game/Materials/M_Blue.M_Blue")))

(event Collision|EventActorBeginOverlap
  (params (OtherActor :type Actor%20Object%20Reference)))

(event EventTick
  (params (DeltaSeconds :type Float%20%28single-precision%29)))

(fn ConstructionScript)

(fn GetInteractionText
  (return (select (Variables|Default|GetPressed) "Кнопка нажата" "Нажать на кнопку") (Variables|Default|GetPressed)))

(fn Interact
  (params (owner :type Pawn%20Object%20Reference))
  (Utilities|Casting|CastToBP_2DCharacter owner
    (:then
      (if (Variables|Default|GetPressed)
        (return false)
        (else
          (Class|INAction|Action(Message) (Variables|Default|GetActionActor))
          (Rendering|Material|SetMaterial (Variables|Default|GetboxModel) 0 "/Game/Materials/M_Green.M_Green")
          (Variables|Default|SetPressed true)
          (CallFunction|PressEvent)
          (return true))))
    (:CastFailed
      (return false))))