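; BP_LegsButton is an interactable button actor that is visible and collidable only while the game is in 3D view.
; It binds to BP_Gamemode's view-change dispatchers on BeginPlay, showing or hiding its Cube and toggling that mesh's collision.
; Its Box overlap registers the actor as the BP_3DCharacter's LegsButton on entry and clears it on exit; press logic is not in this Blueprint.
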(event OnComponentBeginOverlap(Box)
  (params (OverlappedComponent :type Primitive%20Component%20Object%20Reference) (OtherActor :type Actor%20Object%20Reference) (OtherComp :type Primitive%20Component%20Object%20Reference) (OtherBodyIndex :type Integer) (bFromSweep :type Boolean) (SweepResult :type Hit%20Result%20Structure%20%28by%20ref%29))
  (bind _asbp_3dcharacter (Utilities|Casting|CastToBP_3DCharacter OtherActor))
  (Variables|/Game/Blueprints/Characters/BP_3DCharacter.BP_3DCharacter_C|SetLegsButton _asbp_3dcharacter self))

(event OnComponentEndOverlap(Box)
  (params (OverlappedComponent :type Primitive%20Component%20Object%20Reference) (OtherActor :type Actor%20Object%20Reference) (OtherComp :type Primitive%20Component%20Object%20Reference) (OtherBodyIndex :type Integer))
  (bind _asbp_3dcharacter (Utilities|Casting|CastToBP_3DCharacter OtherActor))
  (Variables|/Game/Blueprints/Characters/BP_3DCharacter.BP_3DCharacter_C|SetLegsButton _asbp_3dcharacter 0))

(event Custom|ChangeViewTo2D
  (params (ViewPlane :type Vector%204%20Structure) (Distanse :type Float%20%28single-precision%29))
  (bind _cube (Variables|Default|GetCube))
  (Development|SetHiddeninGame _cube true false)
  (Collision|SetCollisionEnabled _cube "NoCollision"))

(event Custom|ChangeViewTo3D
  (params (Character :type BP%203D%20Character%20Object%20Reference))
  (bind _cube (Variables|Default|GetCube))
  (Development|SetHiddeninGame _cube false false)
  (Collision|SetCollisionEnabled _cube "QueryAndPhysics"))

(event EventBeginPlay
  (bind _asbp_gamemode (Utilities|Casting|CastToBP_Gamemode (Game|GetGameMode)))
  (EventDispatchers|AssignChangeViewto2D _asbp_gamemode (delegate Custom|ChangeViewTo2D))
  (EventDispatchers|AssignChangeViewto3D _asbp_gamemode (delegate Custom|ChangeViewTo3D)))

(event Collision|EventActorBeginOverlap
  (params (OtherActor :type Actor%20Object%20Reference)))

(event EventTick
  (params (DeltaSeconds :type Float%20%28single-precision%29)))

(fn ConstructionScript)