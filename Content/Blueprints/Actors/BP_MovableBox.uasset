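; BP_MovableBox is a physics box that adapts to the game's switches between 2D and 3D views, broadcast by BP_Gamemode.
; In 2D, boxes close enough to the view plane slide their Box2 component onto it along the normal; others are hidden and lose Box2 collision.
; In 3D, Box2's offset, collision and visibility are restored.
; Mass scales with volume, and construction zeroes rotation.
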(event Custom|ChangeViewTo2D
  (params (ViewPlane :type Vector%204%20Structure) (Distanse :type Float%20%28single-precision%29))
  (bind (_x _y _z) (Math|Vector4|BreakVector4 ViewPlane))
  (bind _returnvalue (Math|Vector|MakeVector _x _y _z))
  (bind _returnvalue_2 (Math|Vector|Normalize _returnvalue))
  (bind _distanse (Utilities|GetDistansetoPlane (Transformation|GetWorldLocation (Variables|Default|GetBox)) ViewPlane))
  (if (< (+ _distanse (Math|Vector|VectorLength (* _returnvalue_2 (Transformation|GetActorScale3D) (Math|Vector|MakeVector 5e+01 5e+01 5e+01)))) Distanse)
    (Collision|SetCollisionEnabled (Variables|Default|GetBox2) "QueryAndPhysics")
    (Rendering|SetActorHiddenInGame false)
    (Transformation|SetRelativeLocation (Variables|Default|GetBox2) (+ (/ (* (* _returnvalue_2 -1.0) _distanse) (Transformation|GetActorScale3D)) "0, 0,10.000000") true true)
    (else
      (Collision|SetCollisionEnabled (Variables|Default|GetBox2) "NoCollision")
      (Rendering|SetActorHiddenInGame true))))

(event Custom|ChangeViewTo3D
  (params (Character :type BP%203D%20Character%20Object%20Reference))
  (Transformation|SetRelativeLocation (Variables|Default|GetBox2) "0, 0,10.000000" true true)
  (Collision|SetCollisionEnabled (Variables|Default|GetBox2) "QueryAndPhysics")
  (Rendering|SetActorHiddenInGame false))

(event EventBeginPlay
  (bind _returnvalue (Transformation|GetActorScale3D))
  (bind (_x _y _z) (Math|Vector|BreakVector _returnvalue))
  (bind _asbp_gamemode (Utilities|Casting|CastToBP_Gamemode (Game|GetGameMode)))
  (EventDispatchers|AssignChangeViewto2D _asbp_gamemode (delegate Custom|ChangeViewTo2D))
  (EventDispatchers|AssignChangeViewto3D _asbp_gamemode (delegate Custom|ChangeViewTo3D))
  (Class|PrimitiveComponent|SetMassOverrideinKg (Variables|Default|GetBox) "None" (* _x _y _z 1e+02) true))

(event Collision|EventActorBeginOverlap
  (params (OtherActor :type Actor%20Object%20Reference)))

(event EventTick
  (params (DeltaSeconds :type Float%20%28single-precision%29)))

(fn ConstructionScript
  (Transformation|SetActorRotation "0, 0, 0"))