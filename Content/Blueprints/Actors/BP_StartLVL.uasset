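; BP_StartLVL is a two-door transition chamber that moves the player between levels.
; With Level set, the trigger or Action raises the in-door, and once it closes with the player inside, LVL_2_full opens.
; The character's offset and rotation relative to the chamber are saved to BP_GameInstands before loading.
; Without Level, entering InsideBox can raise the out-door, and leaving lowers it, both doors using timeline lerps.
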(event OnComponentBeginOverlap(InsideBox)
  (params (OverlappedComponent :type Primitive%20Component%20Object%20Reference) (OtherActor :type Actor%20Object%20Reference) (OtherComp :type Primitive%20Component%20Object%20Reference) (OtherBodyIndex :type Integer) (bFromSweep :type Boolean) (SweepResult :type Hit%20Result%20Structure%20%28by%20ref%29))
  (Variables|Default|SetIsInside true)
  (if (Math|Boolean|ANDBoolean (not (Variables|Default|GetOpenedOut)) (not (Variables|Default|GetOpenedIn)) (not (Utilities|IsValidSoftObjectReference (Variables|Default|GetLevel))))
    (Variables|Default|SetOpenedOut true)
    (bind _lerping (Timeline|OutDoorTImeline Play)
      (:Update
        (Transformation|SetRelativeLocation (Variables|Default|GetOutDoor) (Math|Vector|Lerp(Vector) "0,700.000000,450.000000" "0,700.000000,950.000000" _lerping) false false)))))

(event OnComponentEndOverlap(InsideBox)
  (params (OverlappedComponent :type Primitive%20Component%20Object%20Reference) (OtherActor :type Actor%20Object%20Reference) (OtherComp :type Primitive%20Component%20Object%20Reference) (OtherBodyIndex :type Integer))
  (Variables|Default|SetIsInside false)
  (Variables|Default|SetOpenedOut false)
  (bind _lerping (Timeline|OutDoorTImeline Reverse)
    (:Update
      (Transformation|SetRelativeLocation (Variables|Default|GetOutDoor) (Math|Vector|Lerp(Vector) "0,700.000000,450.000000" "0,700.000000,950.000000" _lerping) false false))))

(event OnComponentEndOverlap(Trigger)
  (params (OverlappedComponent :type Primitive%20Component%20Object%20Reference) (OtherActor :type Actor%20Object%20Reference) (OtherComp :type Primitive%20Component%20Object%20Reference) (OtherBodyIndex :type Integer))
  (bind _returnvalue (Game|GetGameMode))
  (bind _asbp_gamemode (Utilities|Casting|CastToBP_Gamemode _returnvalue))
  (bind _3dcharacter (Variables|/Game/Blueprints/GameRules/BP_Gamemode.BP_Gamemode_C|Get3DCharacter _asbp_gamemode))
  (if (Variables|Default|GetIsInside)
    (Variables|Default|SetOpenedIn false)
    (bind _lerping (Timeline|InDoorTimeline Reverse)
      (:Update
        (Transformation|SetRelativeLocation (Variables|Default|GetInDoor) (Math|Vector|Lerp(Vector) "0,-700.000000,450.000000" "0,-700.000000,950.000000" _lerping) false false))
      (:Finished
        (if (and (not (Variables|Default|GetOpenedIn)) (Variables|Default|GetIsInside))
          (bind _asbp_game_instands (Utilities|Casting|CastToBP_GameInstands (Game|GetGameInstance)))
          (Variables|/Game/Blueprints/GameRules/BP_GameInstands.BP_GameInstands_C|SetRelLocation _asbp_game_instands (- (Transformation|GetActorLocation _3dcharacter) (Transformation|GetActorLocation)))
          (Variables|/Game/Blueprints/GameRules/BP_GameInstands.BP_GameInstands_C|SetRelRotator _asbp_game_instands (Math|Rotator|Delta(Rotator) (Transformation|GetActorRotation _3dcharacter) (Transformation|GetActorRotation)))
          (Game|OpenLevel(byObjectReference) "/Game/Blueprints/Maps/LVL_2_full.LVL_2_full"))))))

(event OnComponentBeginOverlap(Trigger)
  (params (OverlappedComponent :type Primitive%20Component%20Object%20Reference) (OtherActor :type Actor%20Object%20Reference) (OtherComp :type Primitive%20Component%20Object%20Reference) (OtherBodyIndex :type Integer) (bFromSweep :type Boolean) (SweepResult :type Hit%20Result%20Structure%20%28by%20ref%29))
  (bind _returnvalue (Game|GetGameMode))
  (bind _asbp_gamemode (Utilities|Casting|CastToBP_Gamemode _returnvalue))
  (bind _3dcharacter (Variables|/Game/Blueprints/GameRules/BP_Gamemode.BP_Gamemode_C|Get3DCharacter _asbp_gamemode))
  (if (Utilities|IsValidSoftObjectReference (Variables|Default|GetLevel))
    (Variables|Default|SetOpenedIn true)
    (bind _lerping (Timeline|InDoorTimeline Play)
      (:Update
        (Transformation|SetRelativeLocation (Variables|Default|GetInDoor) (Math|Vector|Lerp(Vector) "0,-700.000000,450.000000" "0,-700.000000,950.000000" _lerping) false false))
      (:Finished
        (if (and (not (Variables|Default|GetOpenedIn)) (Variables|Default|GetIsInside))
          (bind _asbp_game_instands (Utilities|Casting|CastToBP_GameInstands (Game|GetGameInstance)))
          (Variables|/Game/Blueprints/GameRules/BP_GameInstands.BP_GameInstands_C|SetRelLocation _asbp_game_instands (- (Transformation|GetActorLocation _3dcharacter) (Transformation|GetActorLocation)))
          (Variables|/Game/Blueprints/GameRules/BP_GameInstands.BP_GameInstands_C|SetRelRotator _asbp_game_instands (Math|Rotator|Delta(Rotator) (Transformation|GetActorRotation _3dcharacter) (Transformation|GetActorRotation)))
          (Game|OpenLevel(byObjectReference) "/Game/Blueprints/Maps/LVL_2_full.LVL_2_full"))))))

(event Custom|OpenOutDoorEvent
  (bind _lerping (Timeline|OutDoorTImeline Play)
    (:Update
      (Transformation|SetRelativeLocation (Variables|Default|GetOutDoor) (Math|Vector|Lerp(Vector) "0,700.000000,450.000000" "0,700.000000,950.000000" _lerping) false false))))

(event EventAction
  (bind _returnvalue (Game|GetGameMode))
  (bind _asbp_gamemode (Utilities|Casting|CastToBP_Gamemode _returnvalue))
  (bind _3dcharacter (Variables|/Game/Blueprints/GameRules/BP_Gamemode.BP_Gamemode_C|Get3DCharacter _asbp_gamemode))
  (if (Utilities|IsValidSoftObjectReference (Variables|Default|GetLevel))
    (Variables|Default|SetOpenedIn true)
    (bind _lerping (Timeline|InDoorTimeline Play)
      (:Update
        (Transformation|SetRelativeLocation (Variables|Default|GetInDoor) (Math|Vector|Lerp(Vector) "0,-700.000000,450.000000" "0,-700.000000,950.000000" _lerping) false false))
      (:Finished
        (if (and (not (Variables|Default|GetOpenedIn)) (Variables|Default|GetIsInside))
          (bind _asbp_game_instands (Utilities|Casting|CastToBP_GameInstands (Game|GetGameInstance)))
          (Variables|/Game/Blueprints/GameRules/BP_GameInstands.BP_GameInstands_C|SetRelLocation _asbp_game_instands (- (Transformation|GetActorLocation _3dcharacter) (Transformation|GetActorLocation)))
          (Variables|/Game/Blueprints/GameRules/BP_GameInstands.BP_GameInstands_C|SetRelRotator _asbp_game_instands (Math|Rotator|Delta(Rotator) (Transformation|GetActorRotation _3dcharacter) (Transformation|GetActorRotation)))
          (Game|OpenLevel(byObjectReference) "/Game/Blueprints/Maps/LVL_2_full.LVL_2_full"))))))

(event Collision|EventActorBeginOverlap
  (params (OtherActor :type Actor%20Object%20Reference)))

(event EventTick
  (params (DeltaSeconds :type Float%20%28single-precision%29)))

(event EventBeginPlay
  (Variables|Default|SetIsInside (Utilities|IsValidSoftObjectReference (Variables|Default|GetLevel))))

(fn ConstructionScript)