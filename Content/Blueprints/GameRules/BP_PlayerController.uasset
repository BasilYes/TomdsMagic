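; BP_PlayerController is the player controller that creates and manages the interact, fast menu and target HUD widgets.
; It binds to BP_Gamemode's view-change events, hiding the target widget in 2D view and restoring it in 3D.
; The Menu input refreshes the fast menu widget, and possessing a BP_MoveCamPawn removes the interact widget from the viewport.
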(event Custom|ChangeViewTo2D_Event_0
  (params (ViewPlane :type Vector%204%20Structure) (Distanse :type Float%20%28single-precision%29))
  (Widget|RemovefromParent (Variables|Default|GetTarget)))

(event Custom|ChangeViewTo3D_Event_0
  (params (Character :type BP%203D%20Character%20Object%20Reference))
  (UserInterface|Viewport|AddtoViewport (Variables|Default|GetTarget) 0))

(event EventBeginPlay
  (bind _returnvalue (UserInterface|CreateWidget "/Game/Blueprints/Widgets/W_Interact.W_Interact_C" self))
  (Variables|Default|Setinteract_widget _returnvalue)
  (bind _returnvalue_2 (UserInterface|CreateWidget "/Game/Blueprints/Widgets/W_FastMenu.W_FastMenu_C" self))
  (Variables|Default|SetMenu _returnvalue_2)
  (bind _returnvalue_3 (UserInterface|CreateWidget "/Game/Blueprints/Widgets/W_Target.W_Target_C" self))
  (bind _output_get (Variables|Default|SetTarget _returnvalue_3))
  (UserInterface|Viewport|AddtoViewport _output_get 0)
  (bind _asbp_gamemode (Utilities|Casting|CastToBP_Gamemode (Game|GetGameMode)))
  (EventDispatchers|AssignChangeViewto2D _asbp_gamemode (delegate Custom|ChangeViewTo2D_Event_0))
  (EventDispatchers|AssignChangeViewto3D _asbp_gamemode (delegate Custom|ChangeViewTo3D_Event_0)))

(event EventTick
  (params (DeltaSeconds :type Float%20%28single-precision%29)))

(event EventPossess
  (params (PossessedPawn :type Pawn%20Object%20Reference))
  (Utilities|Casting|CastToBP_MoveCamPawn PossessedPawn)
  (Utilities|IsValid (Variables|Default|Getinteract_widget)
    (:Is%20Valid
      (if (UserInterface|Viewport|IsinViewport (Variables|Default|Getinteract_widget))
        (Widget|RemovefromParent (Variables|Default|Getinteract_widget))))))

(event Input|ActionEvents|InputActionMenu
  (params (Key :type Key%20Structure :default "None"))
  (:Pressed
    (Default|UpdateWidget (Variables|Default|GetMenu))))

(fn ConstructionScript)