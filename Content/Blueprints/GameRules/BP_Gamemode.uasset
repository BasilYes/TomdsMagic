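; Game mode that switches play between the 3D character and a side-view 2D character at a target.
; Each switch possesses a temporary BP_MoveCamPawn for a two-second camera transition, then hands control to the destination character.
; Entering 2D requires a valid LegsButton, whose horizontal distance to the target sets orthographic width and camera offset.
; View-change calls announce each switch, passing a plane computed by PlaneEquation and that distance for 2D.
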(event Custom|ChangeTo2D
  (params (Target :type BP%20Wall%20Eye%20Object%20Reference))
  (bind _returnvalue (Transformation|GetActorLocation Target))
  (bind _returnvalue_2 (Transformation|GetActorScale3D Target))
  (bind _3dcharacter (Variables|Default|Get3DCharacter))
  (bind _3dcharacter_2 (Variables|Default|Get3DCharacter))
  (bind _3dcharacter_3 (Variables|Default|Get3DCharacter))
  (bind _3dcharacter_4 (Variables|Default|Get3DCharacter))
  (bind _3dcharacter_5 (Variables|Default|Get3DCharacter))
  (bind (_x _y) (Math|Vector|BreakVector _returnvalue))
  (bind _camera (Variables|/Game/Blueprints/Characters/BP_3DCharacter.BP_3DCharacter_C|GetCamera _3dcharacter_2))
  (bind _legsbutton (Variables|/Game/Blueprints/Characters/BP_3DCharacter.BP_3DCharacter_C|GetLegsButton _3dcharacter_3))
  (bind _legsbutton_2 (Variables|/Game/Blueprints/Characters/BP_3DCharacter.BP_3DCharacter_C|GetLegsButton _3dcharacter_5))
  (bind _returnvalue_3 (Transformation|GetActorTransform _legsbutton))
  (bind _returnvalue_4 (Transformation|GetActorLocation _legsbutton_2))
  (bind _returnvalue_5 (Math|Vector2D|MakeVector2D _x _y))
  (bind _returnvalue_6 (Transformation|GetWorldTransform _camera))
  (bind (_location _rotation _scale) (Math|Transform|BreakTransform _returnvalue_3))
  (bind (_x_2 _y_2) (Math|Vector|BreakVector _returnvalue_4))
  (bind (_x_3 _y_3) (Math|Vector|BreakVector _location))
  (bind _returnvalue_7 (Math|Vector2D|MakeVector2D _x_2 _y_2))
  (bind _returnvalue_8 (- _returnvalue_7 _returnvalue_5))
  (bind _returnvalue_9 (Math|Vector2D|Vector2DLength _returnvalue_8))
  (Utilities|IsValid _legsbutton
    (:Is%20Valid
      (bind _returnvalue_10 (Game|SpawnActorfromClass "/Game/Blueprints/Characters/BP_MoveCamPawn.BP_MoveCamPawn_C" _returnvalue_6 "AlwaysSpawn" _3dcharacter_4 _returnvalue_6 (Math|Transform|MakeTransform (Math|Vector|MakeVector _x_3 _y_3 (.Z (Math|Vector|BreakVector (Transformation|GetWorldLocation (Variables|/Game/Blueprints/Actors/Interactable/BP_WallEye.BP_WallEye_C|GetBox Target))))) _rotation _scale) _3dcharacter_4))
      (Pawn|Possess (Pawn|GetController (Variables|Default|Get3DCharacter)) _returnvalue_10)
      (Utilities|FlowControl|Delay 2.0)
      (bind _returnvalue_11 (Game|SpawnActorfromClass "/Game/Blueprints/Characters/BP_2DCharacter.BP_2DCharacter_C" (Math|Transform|MakeTransform (+ (Transformation|GetActorLocation Target) (* _returnvalue_2 (Math|Vector|MakeVector 0.0 0.0 88.0))) (Transformation|GetActorRotation Target) _returnvalue_2) "Undefined" _3dcharacter _3dcharacter))
      (Pawn|Possess (Pawn|GetController _returnvalue_10) _returnvalue_11)
      (Actor|DestroyActor _returnvalue_10)
      (Class|CameraComponent|SetOrthoWidth (Variables|/Game/Blueprints/Characters/BP_2DCharacter.BP_2DCharacter_C|GetCamera _returnvalue_11) (* (Variables|/Script/Engine.CameraComponent|GetAspectRatio (Variables|/Game/Blueprints/Characters/BP_2DCharacter.BP_2DCharacter_C|GetCamera _returnvalue_11)) _returnvalue_9))
      (Transformation|SetRelativeLocation (Variables|/Game/Blueprints/Characters/BP_2DCharacter.BP_2DCharacter_C|GetCamera _returnvalue_11) (/ (Math|Vector|MakeVector (- 0.0 _returnvalue_9) (.y (Variables|/Script/Engine.SceneComponent|GetRelativeLocation (Variables|/Game/Blueprints/Characters/BP_2DCharacter.BP_2DCharacter_C|GetCamera _returnvalue_11))) (.z (Variables|/Script/Engine.SceneComponent|GetRelativeLocation (Variables|/Game/Blueprints/Characters/BP_2DCharacter.BP_2DCharacter_C|GetCamera _returnvalue_11)))) (Transformation|GetActorScale3D _returnvalue_11)) false false)
      (Variables|Default|SetIs2D true)
      (Default|CallChangeViewto2D (CallFunction|PlaneEquation (Transformation|GetActorLocation Target) "0, 0,1.000000" (Math|Vector|CrossProduct (Transformation|GetActorForwardVector Target) "0, 0,1.000000")) _returnvalue_9))))

(event Custom|ChangeTo3D
  (params (2DCharacter :type BP%202D%20Character%20Object%20Reference))
  (bind _camera (Variables|/Game/Blueprints/Characters/BP_2DCharacter.BP_2DCharacter_C|GetCamera 2DCharacter))
  (bind _3dcharacter (Variables|Default|Get3DCharacter))
  (bind _3dcharacter_2 (Variables|Default|Get3DCharacter))
  (bind _3dcharacter_3 (Variables|Default|Get3DCharacter))
  (bind _returnvalue (Transformation|GetWorldLocation _camera))
  (bind _returnvalue_2 (Transformation|GetWorldRotation _camera))
  (bind _camera_2 (Variables|/Game/Blueprints/Characters/BP_3DCharacter.BP_3DCharacter_C|GetCamera _3dcharacter))
  (bind _returnvalue_3 (Math|Transform|MakeTransform _returnvalue _returnvalue_2))
  (Default|CallChangeViewto3D (Variables|Default|Get3DCharacter))
  (bind _returnvalue_4 (Game|SpawnActorfromClass "/Game/Blueprints/Characters/BP_MoveCamPawn.BP_MoveCamPawn_C" _returnvalue_3 "AlwaysSpawn" _3dcharacter_2 _returnvalue_3 (Math|Transform|MakeTransform (Transformation|GetWorldLocation _camera_2) (Transformation|GetWorldRotation _camera_2)) _3dcharacter_2))
  (Pawn|Possess (Pawn|GetController 2DCharacter) _returnvalue_4)
  (Actor|DestroyActor 2DCharacter)
  (Utilities|FlowControl|Delay 2.0)
  (Pawn|Possess (Pawn|GetController _returnvalue_4) (Variables|Default|Get3DCharacter))
  (Pawn|SetControlRotation (Pawn|GetController _3dcharacter_3) (Transformation|GetWorldRotation (Variables|/Game/Blueprints/Characters/BP_3DCharacter.BP_3DCharacter_C|GetCamera _3dcharacter_3)))
  (Actor|DestroyActor _returnvalue_4)
  (Variables|Default|SetIs2D false))

(fn ConstructionScript)

(fn PlaneEquation
  (params (Point :type Vector) (vec1 :type Vector) (vec2 :type Vector))
  (bind (_x _y _z) (Math|Vector|BreakVector Point))
  (bind (_x_2 _y_2 _z_2) (Math|Vector|BreakVector vec1))
  (bind (_x_3 _y_3 _z_3) (Math|Vector|BreakVector vec2))
  (bind _returnvalue (* _z_2 _x_3 -1.0))
  (bind _returnvalue_2 (* _x_2 _y_3))
  (bind _returnvalue_3 (* _y_2 _x_3 -1.0))
  (bind _returnvalue_4 (* _y_2 _z_3))
  (bind _returnvalue_5 (* _z_2 _y_3 -1.0))
  (bind _returnvalue_6 (* _x_2 _z_3))
  (bind _returnvalue_7 (+ _returnvalue_6 _returnvalue))
  (bind _returnvalue_8 (+ _returnvalue_2 _returnvalue_3))
  (bind _returnvalue_9 (+ _returnvalue_4 _returnvalue_5))
  (bind _returnvalue_10 (* _returnvalue_8 -1.0))
  (bind _returnvalue_11 (* _returnvalue_9 -1.0))
  (return (Math|Vector4|MakeVector4 _returnvalue_11 _returnvalue_7 _returnvalue_10 (* (+ (* _x _returnvalue_11) (* _y _returnvalue_7) (* _z _returnvalue_10)) -1.0))))